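; Actor Blueprint that drives a robotic arm skeletal mesh through a Control Rig component, following a target actor's transform.
; The component takes initial bone transforms from the mesh asset during pre-construction and maps the complete skeletal mesh after initialization.
; Before each forwards solve, it copies Target1's transform into the RoboticArmModel_CtrlRig1 Target variable, printing a message if the target or cast is invalid.
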(event `self.ControlRig.OnPreConstructionDelegate`
  (params (Component :type "ControlRigComponent Object Reference"))
  (`ControlRigComponent.SetBoneInitialTransformsFromSkeletalMesh` (`self.ControlRig`) (`SkeletalMeshComponent.GetSkeletalMeshAsset` (`self.SkeletalMesh`))))

(event `self.ControlRig.OnPostInitializeDelegate`
  (params (Component :type "ControlRigComponent Object Reference"))
  (`ControlRigComponent.AddMappedCompleteSkeletalMesh` (`self.ControlRig`) (`self.SkeletalMesh`)))

(event `self.ControlRig.OnPreForwardsSolveDelegate`
  (params (Component :type "ControlRigComponent Object Reference"))
  (bind _target1 (`self.Target1`))
  (bind _asrobotic_arm_model_ctrl_rig_1 (cast `/Game/SimBlank/Arm/Assets/ArmRig/RoboticArmModel_CtrlRig1` (`ControlRigComponent.GetControlRig` Component))
    (:`then`
      (`/Engine/EditorBlueprintResources/StandardMacros.IsValid` _target1
        (:`Is Valid`
          (set `/Game/SimBlank/Arm/Assets/ArmRig/RoboticArmModel_CtrlRig1.Target` (`self.GetTransform` _target1) _asrobotic_arm_model_ctrl_rig_1))
        (:`Is Not Valid`
          (`KismetSystemLibrary.PrintText` "Target 1 is empty"))))
    (:`CastFailed`
      (`KismetSystemLibrary.PrintText` "Could not cast to RoboticAmr ctrl rig"))))

(fn `UserConstructionScript`)